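; BP_WheelMove is an actor that moves its Cube component around a square loop in the local XZ plane while spinning it like a wheel.
; Each tick it switches on the Movwtype direction state, calls the matching move function scaled by Speed, and applies a negative pitch world rotation.
; Each move function advances the state when the relative position reaches its bound, cycling Right, Up, Left, Down.
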(event `self.ReceiveTick`
  (params (DeltaSeconds :type "Float (single-precision)"))
  (bind _cube (`self.Cube`))
  (bind _returnvalue (* DeltaSeconds (`self.speed`)))
  (switch `/Game/EN_movetype` (`self.Movwtype`)
    (:`NewEnumerator0`
      (`self.MoveRight!` _returnvalue)
      (`SceneComponent.K2_AddWorldRotation` _cube (`KismetMathLibrary.MakeRotator` 0.0 (* _returnvalue -1.0)) false false))
    (:`NewEnumerator1`
      (`self.MoveUp!` _returnvalue)
      (`SceneComponent.K2_AddWorldRotation` _cube (`KismetMathLibrary.MakeRotator` 0.0 (* _returnvalue -1.0)) false false))
    (:`NewEnumerator2`
      (`self.MoveLeft!` _returnvalue)
      (`SceneComponent.K2_AddWorldRotation` _cube (`KismetMathLibrary.MakeRotator` 0.0 (* _returnvalue -1.0)) false false))
    (:`NewEnumerator3`
      (`self.MoveDown!` _returnvalue)
      (`SceneComponent.K2_AddWorldRotation` _cube (`KismetMathLibrary.MakeRotator` 0.0 (* _returnvalue -1.0)) false false))))

(fn `MoveDown!`
  (params (A :type "Float (double-precision)"))
  (bind _cube (`self.Cube`))
  (bind (_relativelocation_x _relativelocation_y _relativelocation_z) (`KismetMathLibrary.BreakVector` (`SceneComponent.RelativeLocation` _cube)))
  (`SceneComponent.K2_AddRelativeLocation` _cube (`KismetMathLibrary.MakeVector` 0.0 0.0 (* A -1.0)) false false)
  (if (<= _relativelocation_z 0.0)
    (set `self.Movwtype` "NewEnumerator0")))

(fn `MoveLeft!`
  (params (A :type "Float (double-precision)"))
  (bind _cube (`self.Cube`))
  (bind _relativelocation_x (`KismetMathLibrary.BreakVector` (`SceneComponent.RelativeLocation` _cube)))
  (`SceneComponent.K2_AddRelativeLocation` _cube (`KismetMathLibrary.MakeVector` (* A -1.0)) false false)
  (if (<= _relativelocation_x 0.0)
    (set `self.Movwtype` "NewEnumerator3")))

(fn `MoveRight!`
  (params (DeltaLocation_X :type "Float (double-precision)"))
  (bind _cube (`self.Cube`))
  (bind _relativelocation_x (`KismetMathLibrary.BreakVector` (`SceneComponent.RelativeLocation` _cube)))
  (`SceneComponent.K2_AddRelativeLocation` _cube (`KismetMathLibrary.MakeVector` DeltaLocation_X) false false)
  (if (>= _relativelocation_x 500.0)
    (set `self.Movwtype` "NewEnumerator1")))

(fn `MoveUp!`
  (params (DeltaLocation_Z :type "Float (double-precision)"))
  (bind _cube (`self.Cube`))
  (bind (_relativelocation_x _relativelocation_y _relativelocation_z) (`KismetMathLibrary.BreakVector` (`SceneComponent.RelativeLocation` _cube)))
  (`SceneComponent.K2_AddRelativeLocation` _cube (`KismetMathLibrary.MakeVector` 0.0 0.0 DeltaLocation_Z) false false)
  (if (>= _relativelocation_z 500.0)
    (set `self.Movwtype` "NewEnumerator2")))

(fn `UserConstructionScript`)