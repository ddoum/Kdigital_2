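; BP_DirtyTimer is a rough count-up timer that prints its elapsed time as a debug string every frame.
; Tick accumulates DeltaSeconds at ten times speed into TotalSec, then floors the division and modulo by 60 to get minutes and seconds.
; The printout uses Korean 분/초 units and omits minutes below one minute.
; The FloatToStr분초 function is an unfinished, empty stub that the event graph does not call.
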(event `self.ReceiveTick`
  (params (DeltaSeconds :type "Float (single-precision)"))
  (bind _output_get (set `self.TotalSec` (+ (* DeltaSeconds 10.0) (`self.TotalSec`))))
  (bind _returnvalue (`KismetMathLibrary.FFloor` (/ _output_get 60.0)))
  (if (> _returnvalue 0)
    (bind _returnvalue_2 (`KismetMathLibrary.FFloor` (mod _output_get 60.0)))
    (`KismetSystemLibrary.PrintString` (`KismetStringLibrary.Concat_StrStr` (`KismetStringLibrary.Conv_IntToString` _returnvalue) "분" (`KismetStringLibrary.Conv_IntToString` _returnvalue_2) "초"))
    (else
      (`KismetSystemLibrary.PrintString` (`KismetStringLibrary.Concat_StrStr` (`KismetStringLibrary.Conv_IntToString` _returnvalue_2) "초")))))

(fn `FloatToStr분초`
  (params (minute :type "Float (double-precision)")))

(fn `UserConstructionScript`)